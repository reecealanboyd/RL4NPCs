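; Weapon Blueprint that spawns a Projectile at its ProjectileSpawnPoint, built for automatic fire but marked "Unused at the moment" at PullTrigger.
; PullTrigger passes a DoOnce to fire immediately and set a looping Fire timer from RoundsPerSecond, converting to float only after the division.
; ReleaseTrigger resets the DoOnce, but its timer clear has an empty function name, so it does not target the Fire timer.
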(event `PullTrigger`
  ;[1 1 1] Unused at the moment
  (`/Engine/EditorBlueprintResources/StandardMacros.DoOnce` false :!label _label
    (:`Completed`
      (`self.Fire`)
      (`KismetSystemLibrary.K2_SetTimer` null "Fire" (`KismetMathLibrary.Conv_IntToDouble` (/ 1 (`self.RoundsPerSecond`))) true))))

(event `ReleaseTrigger`
  ;[1 1 1] Unused at the moment
  (`KismetSystemLibrary.K2_ClearTimer` null)
  (goto _label :!via `Reset`))

(event `Fire`
  (`|SpawnActorFromClass` "/Game/Blueprints/Projectile.Projectile_C" (`SceneComponent.K2_GetComponentToWorld` (`self.ProjectileSpawnPoint`)) "Undefined" "OverrideRootScale"))

(fn `UserConstructionScript`)
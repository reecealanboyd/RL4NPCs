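; AI-driven hero character for Capture the Flag, apparently an RL agent, that spawns its gun and respawns through the game mode on death.
; Perception, hearing and damage events set blackboard flags.
; After each delay, Tick encodes those flags and low health as a printed binary state string.
; It then picks a random action independent of that state: shooting, moving, focus changes or chained EQS queries to hide from an AICharacter.
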(event `self.AIPerception.OnTargetPerceptionUpdated`
  (params (Actor :type "Actor Object Reference") (Stimulus :type "AIStimulus Structure"))
  ;[1 1 1] Flips the flag for seeing the Player
  (cast `/Game/AI/AICharacter` Actor)
  (`BlackboardComponent.SetValueAsBool` (`AIBlueprintHelperLibrary.GetBlackboard` null) "CanSeeRLCharacter" (`.bSuccessfullySensed` (break `AIStimulus` Stimulus))))

(event `/Game/Blueprints/IDamageable.AffectHealth`
  (params (Delta :type "Float (single-precision)"))
  (bind _capsulecomponent (`self.CapsuleComponent`))
  (`BlackboardComponent.SetValueAsBool` (`AIBlueprintHelperLibrary.GetBlackboard` null) "TakingHits" true)
  (`self.CalculateHealth` Delta)
  (if (`self.isDead`)
    (`PrimitiveComponent.SetCollisionResponseToChannel` _capsulecomponent "ECC_WorldDynamic" "ECR_Ignore")
    (`PrimitiveComponent.SetCollisionResponseToChannel` _capsulecomponent "ECC_Pawn" "ECR_Ignore")
    (`self.DetachFromControllerPendingDestroy`)
    (`self.K2_DestroyActor` (`self.Weapon`))
    (`KismetSystemLibrary.Delay` 3.0)
    (`/Game/Blueprints/CaptureTheFlag.RespawnRLCharacter` (`self.GameMode`))
    (`self.K2_DestroyActor` self)))

(event `self.ReceiveActorBeginOverlap`
  (params (OtherActor :type "Actor Object Reference")))

(event `self.ReceiveBeginPlay`
  (bind _guntemp (`self.GunTemp`))
  ;[1 1 1] Attach Gun (Rather poorly) to Character
  (`|ExecutionSequence`
    (:`then_0`
      (bind _returnvalue (`|SpawnActorFromClass` "/Game/Blueprints/Weapon.Weapon_C" (`SceneComponent.K2_GetComponentToWorld` _guntemp) "Undefined" "OverrideRootScale"))
      (bind _output_get (set `self.Weapon` _returnvalue))
      (`self.K2_AttachToComponent` _output_get _guntemp "None" "KeepWorld" "KeepRelative" "KeepWorld" true))
    (:`then_1`
      (bind _ascapture_the_flag (cast `/Game/Blueprints/CaptureTheFlag` (`GameplayStatics.GetGameMode`)))
      (bind _output_get_2 (set `self.GameMode` _ascapture_the_flag))
      (set `/Game/Blueprints/CaptureTheFlag.RLSpawnTransform` (`self.GetTransform`) _output_get_2))))

(event `self.ReceiveTick`
  (params (DeltaSeconds :type "Float (single-precision)"))
  (bind _statestringarray (`self.StateStringArray`))
  (bind _returnvalue (`AIBlueprintHelperLibrary.GetBlackboard` self))
  (`KismetSystemLibrary.Delay` (`self.SelectNewActionTime`))
  (set `self.CurrentState` "\"\"")
  (`KismetArrayLibrary.Array_Clear` _statestringarray)
  (if (`BlackboardComponent.GetValueAsBool` _returnvalue "TakingHits")
    (`KismetArrayLibrary.Array_Add` _statestringarray "1")
    (else
      (`KismetArrayLibrary.Array_Add` _statestringarray "0")))
  (if (`BlackboardComponent.GetValueAsBool` _returnvalue "CanSeeRLCharacter")
    (`KismetArrayLibrary.Array_Add` _statestringarray "1")
    (else
      (`KismetArrayLibrary.Array_Add` _statestringarray "0")))
  (if (`BlackboardComponent.GetValueAsBool` _returnvalue "CanHearEnemy")
    (`KismetArrayLibrary.Array_Add` _statestringarray "1")
    (else
      (`KismetArrayLibrary.Array_Add` _statestringarray "0")))
  (if (<= (`self.health`) 30.0)
    (`KismetArrayLibrary.Array_Add` _statestringarray "1")
    (else
      (`KismetArrayLibrary.Array_Add` _statestringarray "0")))
  (set `self.CurrentState` (`KismetStringLibrary.JoinStringArray` _statestringarray ""))
  (`KismetSystemLibrary.PrintString` (`self.CurrentState`))
  (switch `int` (`KismetMathLibrary.RandomIntegerInRange` 0 6)
    (:`0`
      (`self.ShootWeapon`))
    (:`1`
      (`self.FindRandomLocation`))
    (:`2`
      (`self.FocusOnAICharacter`))
    (:`3`
      (`self.MoveNearAICharacter`))
    (:`4`
      (`self.StopShooting`))
    (:`5`
      (`self.ClearFocus`))
    (:`6`
      (bind _returnvalue_2 (`AIBlueprintHelperLibrary.GetAIController` self))
      (bind _returnvalue_3 (`EnvQueryManager.RunEQSQuery` "/Game/AI/FindAICharacter.FindAICharacter" _returnvalue_2 "SingleResult"))
      (add `EnvQueryInstanceBlueprintWrapper.OnQueryFinishedEvent` _returnvalue_3 (delegate `FindAICharacterQueryFinished`)))))

(event `self.PawnSensing.OnHearNoise`
  (params (Instigator :type "Pawn Object Reference") (Location :type "Vector Structure (by ref)") (Volume :type "Float (single-precision)"))
  (bind _returnvalue (`AIBlueprintHelperLibrary.GetBlackboard` null))
  (`BlackboardComponent.SetValueAsObject` _returnvalue "EnemyHeard" Instigator)
  (`BlackboardComponent.SetValueAsBool` _returnvalue "CanHearEnemy" true)
  (bind _asactor (cast `Actor` (`BlackboardComponent.GetValueAsObject` _returnvalue "EnemyHeard"))))

(event `FindAICharacterQueryFinished`
  (params (QueryInstance :type "EnvQueryInstanceBlueprintWrapper Object Reference") (QueryStatus :type "EEnvQueryStatus Enum"))
  (`BlackboardComponent.SetValueAsObject` (`AIBlueprintHelperLibrary.GetBlackboard` self) "Enemy" (`KismetArrayLibrary.Array_Get` (`EnvQueryInstanceBlueprintWrapper.GetResultsAsActors` QueryInstance)))
  (bind _returnvalue (`EnvQueryManager.RunEQSQuery` "/Game/AI/FindHidingSpotFromAI.FindHidingSpotFromAI" (stale `self.ReceiveTick` _returnvalue_2) "SingleResult"))
  (add `EnvQueryInstanceBlueprintWrapper.OnQueryFinishedEvent` _returnvalue (delegate `FindHidingSpotFromAIQueryFinished`)))

(event `FindHidingSpotFromAIQueryFinished`
  (params (QueryInstance :type "EnvQueryInstanceBlueprintWrapper Object Reference") (QueryStatus :type "EEnvQueryStatus Enum"))
  (`NavigationSystem.SimpleMoveToLocation` (stale `self.ReceiveTick` _returnvalue_2) (`KismetArrayLibrary.Array_Get` (`EnvQueryInstanceBlueprintWrapper.GetResultsAsLocations` QueryInstance))))

(fn `ClearFocus`
  ;[1 1 1] Stops the AICharacter from looking at the player
  (bind _returnvalue (`AIBlueprintHelperLibrary.GetAIController` self))
  (`AIController.K2_ClearFocus` _returnvalue))

(fn `FindRandomLocation`
  ;[1 1 1] Moves to a random location within a navigable radius of 6000
  (bind _returnvalue (`AIBlueprintHelperLibrary.GetAIController` self))
  (`AIController.MoveToLocation` _returnvalue (`NavigationSystem.GetRandomPointInNavigableRadius` (`self.K2_GetActorLocation` (`Controller.K2_GetPawn` _returnvalue)) 6000.0) -1.0 true true true true null true))

(fn `FocusOnAICharacter`
  ;[1 1 1] Makes AICharacter look at the player
  (bind _outactors (`GameplayStatics.GetAllActorsOfClass` "/Game/AI/AICharacter.AICharacter_C"))
  (for _array_element _outactors
    (bind _returnvalue (`AIBlueprintHelperLibrary.GetAIController` self))
    (`AIController.K2_SetFocus` _returnvalue _array_element)))

(fn `MoveNearAICharacter`
  (bind _returnvalue (`AIBlueprintHelperLibrary.GetAIController` self))
  ;[1 1 1] Moves to a random point within 600 units of the RLCharacter
  (bind _outactors (`GameplayStatics.GetAllActorsOfClass` "/Game/AI/AICharacter.AICharacter_C"))
  (for _array_element _outactors
    (`NavigationSystem.SimpleMoveToLocation` _returnvalue (`NavigationSystem.GetRandomPointInNavigableRadius` (`self.K2_GetActorLocation` _array_element) 600.0))))

(fn `ShootWeapon`
  (bind _returnvalue (`AIBlueprintHelperLibrary.GetAIController` self))
  (bind _ashero_character (cast `/Game/Blueprints/HeroCharacter` (`Controller.K2_GetPawn` _returnvalue)))
  (`KismetSystemLibrary.K2_SetTimer` (`/Game/Blueprints/HeroCharacter.Weapon` _ashero_character) "Fire" 0.25 true))

(fn `StopShooting`
  (bind _returnvalue (`AIBlueprintHelperLibrary.GetAIController` self))
  (bind _ashero_character (cast `/Game/Blueprints/HeroCharacter` (`Controller.K2_GetPawn` _returnvalue)))
  (`KismetSystemLibrary.K2_ClearTimer` (`/Game/Blueprints/HeroCharacter.Weapon` _ashero_character) "Fire"))

(fn `UserConstructionScript`)